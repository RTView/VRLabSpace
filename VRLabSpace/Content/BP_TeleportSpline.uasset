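; BP_TeleportSpline is an actor that detects when the VR player leaves any of its three box volumes.
; When the VRPawn's Sphere1 component ends overlap with a box, it calls PlayerIsOut on the pawn.
; It then briefly disables overlap events on all three boxes as a cooldown before re-enabling them.
; Despite the name, its graphs contain no spline or teleport logic.
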(event OnComponentEndOverlap(Box)
  (params (OverlappedComponent :type Primitive%20Component%20Object%20Reference) (OtherActor :type Actor%20Object%20Reference) (OtherComp :type Primitive%20Component%20Object%20Reference) (OtherBodyIndex :type Integer))
  (bind _asvrpawn (Utilities|Casting|CastToVRPawn OtherActor))
  (if (== OtherComp (Variables|/Game/VRTemplate/Blueprints/VRPawn.VRPawn_C|GetSphere1 _asvrpawn))
    (Default|PlayerIsOut _asvrpawn)
    (CallFunction|PauseCollider)))

(event OnComponentEndOverlap(Box1)
  (params (OverlappedComponent :type Primitive%20Component%20Object%20Reference) (OtherActor :type Actor%20Object%20Reference) (OtherComp :type Primitive%20Component%20Object%20Reference) (OtherBodyIndex :type Integer))
  (bind _asvrpawn (Utilities|Casting|CastToVRPawn OtherActor))
  (if (== OtherComp (Variables|/Game/VRTemplate/Blueprints/VRPawn.VRPawn_C|GetSphere1 _asvrpawn))
    (Default|PlayerIsOut _asvrpawn)
    (CallFunction|PauseCollider)))

(event OnComponentEndOverlap(Box2)
  (params (OverlappedComponent :type Primitive%20Component%20Object%20Reference) (OtherActor :type Actor%20Object%20Reference) (OtherComp :type Primitive%20Component%20Object%20Reference) (OtherBodyIndex :type Integer))
  (bind _asvrpawn (Utilities|Casting|CastToVRPawn OtherActor))
  (if (== OtherComp (Variables|/Game/VRTemplate/Blueprints/VRPawn.VRPawn_C|GetSphere1 _asvrpawn))
    (Default|PlayerIsOut _asvrpawn)
    (CallFunction|PauseCollider)))

(event Custom|PauseCollider
  (Variables|/Script/Engine.PrimitiveComponent|SetbGenerateOverlapEvents (Variables|Default|GetBox2) false)
  (Variables|/Script/Engine.PrimitiveComponent|SetbGenerateOverlapEvents (Variables|Default|GetBox) false)
  (Variables|/Script/Engine.PrimitiveComponent|SetbGenerateOverlapEvents (Variables|Default|GetBox1) false)
  (Utilities|FlowControl|Delay 0.5)
  (Variables|/Script/Engine.PrimitiveComponent|SetbGenerateOverlapEvents (Variables|Default|GetBox2) true)
  (Variables|/Script/Engine.PrimitiveComponent|SetbGenerateOverlapEvents (Variables|Default|GetBox) true)
  (Variables|/Script/Engine.PrimitiveComponent|SetbGenerateOverlapEvents (Variables|Default|GetBox1) true))

(event EventBeginPlay)

(event Collision|EventActorBeginOverlap
  (params (OtherActor :type Actor%20Object%20Reference)))

(event EventTick
  (params (DeltaSeconds :type Float%20%28single-precision%29)))

(fn ConstructionScript)